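; Heal potion inventory item that restores the player character's health when used.
; BeginPlay caches the player as an RPG_MainCharacter reference.
; UseItem sets the player's CharacterStats enum, then, if health is below 100, waits briefly before adding the item data's HealAmount, clamped to 0–100, and printing a consumption message.
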(event EventBeginPlay
  (|CallParentFunction)
  (bind _asrpg_main_character (Utilities|Casting|CastToRPG_MainCharacter (Game|GetPlayerCharacter 0)))
  (Variables|Default|SetPlayerRef _asrpg_main_character))

(event Collision|EventActorBeginOverlap
  (params (OtherActor :type Actor%20Object%20Reference))
  (|CallParentFunction OtherActor) ; This node is disabled and will not be called.\nDrag off pins to build functionality.
)

(event EventTick
  (params (DeltaSeconds :type Float%20%28single-precision%29))
  (|CallParentFunction DeltaSeconds))

(event EventUseItem
  (bind _playerref (Variables|Default|GetPlayerRef))
  (Variables|/Game/_Game/Characters/Player/RPG_MainCharacter.RPG_MainCharacter_C|SetCharacterStats _playerref "NewEnumerator1")
  (if (< (Variables|/Game/_Game/Characters/Player/RPG_MainCharacter.RPG_MainCharacter_C|GetCurrentHealth _playerref) 1e+02)
    (Utilities|FlowControl|Delay 0.1)
    (Variables|/Game/_Game/Characters/Player/RPG_MainCharacter.RPG_MainCharacter_C|SetCurrentHealth (Variables|Default|GetPlayerRef) (Math|Float|Clamp(Float) (+ (Variables|/Game/_Game/Characters/Player/RPG_MainCharacter.RPG_MainCharacter_C|GetCurrentHealth _playerref) (.HealAmount (Utilities|Struct|BreakSItemData (Variables|Default|GetItemData)))) 0.0 1e+02))
    (Development|PrintText "Consumed 1 heal potion.")))

(fn ConstructionScript
  (|CallParentFunction))