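; Inventory component for the RPG player, holding item and equipment slot arrays sized from RPGController.
; AddItem stacks up to each item's max, recursing on overflow; other functions use, remove, sell or drop items as physics-enabled Paper2D pickups, merging into existing ones.
; Equip and unequip move items between the arrays and adjust player damage and shield.
; Changes refresh selection-menu slot widgets, and the component also opens the examination widget for items.
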(event Custom|Initialize
  (bind _returnvalue (Game|GetPlayerController 0))
  (bind _asrpgcontroller (Utilities|Casting|CastToRPGController _returnvalue))
  (Utilities|Array|Resize (Variables|Default|GetInventorySlots) (Variables|/Game/_Game/Config/PlayerController/RPGController.RPGController_C|GetInventorySlots _asrpgcontroller))
  (Variables|Default|SetSelectionMenuRef (Variables|/Game/_Game/Config/PlayerController/RPGController.RPGController_C|GetSelectionMenuRef _asrpgcontroller))
  (bind _asrpg_main_character (Utilities|Casting|CastToRPG_MainCharacter (Game|GetPlayerCharacter 0)))
  (Variables|Default|SetPlayerRef _asrpg_main_character)
  (bind _returnvalue_2 (UserInterface|CreateWidget "/Game/_Game/UI/Inventory/W_Examination.W_Examination_C" 0 0))
  (bind _output_get (Variables|Default|SetW_ExaminationRef _returnvalue_2))
  (Variables|/Game/_Game/Config/PlayerController/RPGController.RPGController_C|SetW_ExaminationRef _asrpgcontroller _output_get)
  (bind _outactors (Actor|GetAllActorsOfClass "/Game/_Game/Blueprints/Inventory/ExamineActor/BP_Examination.BP_Examination_C"))
  (Variables|Default|SetBP_ExaminationRef (Utilities|Array|Get(acopy) _outactors))
  (Variables|/Game/_Game/UI/Inventory/W_Examination.W_Examination_C|SetBPC_InventoryRef (Variables|Default|GetW_ExaminationRef) self)
  (Utilities|Array|Resize (Variables|Default|GetEquipSlots) (Variables|/Game/_Game/Config/PlayerController/RPGController.RPGController_C|GetEquipSlots (.AsRPGController (Utilities|Casting|CastToRPGController (Game|GetPlayerController 0))))))

(event Custom|CreateExaminationEquip
  (params (Index :type Integer))
  (bind _selectionmenuref (Variables|Default|GetSelectionMenuRef))
  (bind _w_inventory (Variables|/Game/_Game/UI/Menu/W_SelectionMenu.W_SelectionMenu_C|GetW_Inventory _selectionmenuref))
  (Default|UpdateWidgetforEquip (Variables|Default|GetW_ExaminationRef) Index)
  (Widget|SetVisibility (Variables|Default|GetSelectionMenuRef) "Collapsed")
  (Utilities|IsValid (Variables|/Game/_Game/UI/Inventory/W_Inventory.W_Inventory_C|GetW_InventoryDropDown _w_inventory)
    (:Is%20Valid
      (Default|CloseDropDownMenu _w_inventory))
    (:Is%20Not%20Valid
      _))
  (UserInterface|Viewport|AddtoViewport (Variables|Default|GetW_ExaminationRef) 2))

(event Custom|CreateExaminationWidget
  (params (Index :type Integer))
  (bind _selectionmenuref (Variables|Default|GetSelectionMenuRef))
  (bind _w_inventory (Variables|/Game/_Game/UI/Menu/W_SelectionMenu.W_SelectionMenu_C|GetW_Inventory _selectionmenuref))
  (Default|UpdateWidgetforInventory (Variables|Default|GetW_ExaminationRef) Index)
  (Widget|SetVisibility (Variables|Default|GetSelectionMenuRef) "Collapsed")
  (Utilities|IsValid (Variables|/Game/_Game/UI/Inventory/W_Inventory.W_Inventory_C|GetW_InventoryDropDown _w_inventory)
    (:Is%20Valid
      (Default|CloseDropDownMenu _w_inventory))
    (:Is%20Not%20Valid
      _))
  (UserInterface|Viewport|AddtoViewport (Variables|Default|GetW_ExaminationRef) 2))

(event EventBeginPlay
  (CallFunction|Initialize))

(fn AddItem
  (params (Item :type BP%20Inventory%20Item%20Master%20Class%20Reference) (Amount :type Integer) (Specific%20Free%20Index :type Integer))
  (bind (_success _index) (CallFunction|CheckforEmptySlot))
  (bind (_success_2 _index_2) (CallFunction|CheckforEmptySlot))
  (LocalVariables|SetLocalItem Item)
  (LocalVariables|SetLocalAmount Amount)
  (LocalVariables|SetLocalMaxStackAmount (.MaxStackAmount (Utilities|Struct|BreakSItemData (.ItemData (Utilities|GetClassDefaults (LocalVariables|GetLocalItem))))))
  (if (> (.MaxStackAmount (Utilities|Struct|BreakSItemData (.ItemData (Utilities|GetClassDefaults (LocalVariables|GetLocalItem))))) 1)
    (bind (_success_3 _index_3) (CallFunction|CheckforFreeSlot (LocalVariables|GetLocalItem)))
    (if _success_3
      (LocalVariables|SetLocalIndex _index_3)
      (if (> (+ (.Amount (CallFunction|GetItemDataatIndex (LocalVariables|GetLocalIndex))) (LocalVariables|GetLocalAmount)) (LocalVariables|GetLocalMaxStackAmount))
        (LocalVariables|SetLocalAmount (- (+ (.Amount (CallFunction|GetItemDataatIndex (LocalVariables|GetLocalIndex))) (LocalVariables|GetLocalAmount)) (LocalVariables|GetLocalMaxStackAmount)))
        (Utilities|Array|SetArrayElem (Variables|Default|GetInventorySlots) (LocalVariables|GetLocalIndex) (Utilities|Struct|MakeSInventoryItems (LocalVariables|GetLocalItem) (LocalVariables|GetLocalMaxStackAmount)))
        (CallFunction|UpdateInventorySlot (LocalVariables|GetLocalIndex))
        (bind _remainder (CallFunction|AddItem (LocalVariables|GetLocalItem) (LocalVariables|GetLocalAmount)))
        (return true _remainder)
        (else
          (Utilities|Array|SetArrayElem (Variables|Default|GetInventorySlots) (LocalVariables|GetLocalIndex) (Utilities|Struct|MakeSInventoryItems (LocalVariables|GetLocalItem) (+ (.Amount (CallFunction|GetItemDataatIndex (LocalVariables|GetLocalIndex))) (LocalVariables|GetLocalAmount))))
          (CallFunction|UpdateInventorySlot (LocalVariables|GetLocalIndex))
          (return true 0)))
      (elif _success
        (LocalVariables|SetLocalIndex _index)
        (if (> (LocalVariables|GetLocalAmount) (LocalVariables|GetLocalMaxStackAmount))
          (Utilities|Array|SetArrayElem (Variables|Default|GetInventorySlots) (LocalVariables|GetLocalIndex) (Utilities|Struct|MakeSInventoryItems (LocalVariables|GetLocalItem) (LocalVariables|GetLocalMaxStackAmount)))
          (CallFunction|UpdateInventorySlot (LocalVariables|GetLocalIndex))
          (bind _remainder_2 (CallFunction|AddItem (LocalVariables|GetLocalItem) (- (LocalVariables|GetLocalAmount) (LocalVariables|GetLocalMaxStackAmount))))
          (return true _remainder_2)
          (else
            (Utilities|Array|SetArrayElem (Variables|Default|GetInventorySlots) (LocalVariables|GetLocalIndex) (Utilities|Struct|MakeSInventoryItems (LocalVariables|GetLocalItem) (LocalVariables|GetLocalAmount)))
            (CallFunction|UpdateInventorySlot (LocalVariables|GetLocalIndex))
            (return true 0)))
        (else
          (return false (LocalVariables|GetLocalAmount)))))
    (elif _success_2
      (LocalVariables|SetLocalIndex (+ _index_2 Specific%20Free%20Index))
      (Utilities|Array|SetArrayElem (Variables|Default|GetInventorySlots) (LocalVariables|GetLocalIndex) (Utilities|Struct|MakeSInventoryItems (LocalVariables|GetLocalItem) 1))
      (CallFunction|UpdateInventorySlot (LocalVariables|GetLocalIndex))
      (if (> (- (LocalVariables|GetLocalAmount) 1) 0)
        (bind _remainder_3 (CallFunction|AddItem (LocalVariables|GetLocalItem) (- (LocalVariables|GetLocalAmount) 1)))
        (return true _remainder_3)
        (else
          (return true 0)))
      (else
        (Development|PrintText "No free slots!")
        (return false (LocalVariables|GetLocalAmount))))))

(fn CheckforEmptySlot
  (bind (_array_element _array_index) (Utilities|Array|ForEachLoopwithBreak (Variables|Default|GetInventorySlots) :!label _label)
    (:LoopBody
      (if (Utilities|IsValidClass (.Item (Utilities|Struct|BreakSInventoryItems _array_element)))
        (LocalVariables|SetLocalSuccess false)
        (else
          (LocalVariables|SetLocalSuccess true)
          (LocalVariables|SetLocalIndex _array_index)
          (goto _label Break))))
    (:Completed
      (return (LocalVariables|GetLocalSuccess) (LocalVariables|GetLocalIndex)))))

(fn GetItemDataatIndex
  (params (Index :type Integer))
  (bind _inventoryslots (Variables|Default|GetInventorySlots))
  (bind _output (Utilities|Array|Get(acopy) _inventoryslots Index))
  (bind (_item _amount) (Utilities|Struct|BreakSInventoryItems _output))
  (return _item _amount))

(fn UpdateInventorySlot
  (params (Index :type Integer))
  (Default|UpdateSlot (Utilities|Array|Get(acopy) (Variables|/Game/_Game/UI/Inventory/W_Inventory.W_Inventory_C|GetSlots%20Array (Variables|/Game/_Game/UI/Menu/W_SelectionMenu.W_SelectionMenu_C|GetW_Inventory (Variables|/Game/_Game/Config/PlayerController/RPGController.RPGController_C|GetSelectionMenuRef (.AsRPGController (Utilities|Casting|CastToRPGController (Game|GetPlayerController 0)))))) Index)))

(fn CheckforFreeSlot
  (params (Item :type BP%20Inventory%20Item%20Master%20Class%20Reference))
  (bind (_array_element _array_index) (Utilities|Array|ForEachLoopwithBreak (Variables|Default|GetInventorySlots) :!label _label)
    (:LoopBody
      (if (and (== (.Item (Utilities|Struct|BreakSInventoryItems _array_element)) Item) (< (.Amount (Utilities|Struct|BreakSInventoryItems _array_element)) (.maxstackamount (.ItemData (Utilities|GetClassDefaults Item)))))
        (LocalVariables|SetLocalSuccess true)
        (LocalVariables|SetLocalIndex _array_index)
        (goto _label Break)
        (else
          (LocalVariables|SetLocalSuccess false))))
    (:Completed
      (return (LocalVariables|GetLocalSuccess) (LocalVariables|GetLocalIndex)))))

(fn UseItem
  (params (Index :type Integer))
  (LocalVariables|SetLocalIndex Index)
  (if (> (.Amount (CallFunction|GetItemDataatIndex (LocalVariables|GetLocalIndex))) 0)
    (bind _returnvalue (Actor|GetActorOfClass (.Item (CallFunction|GetItemDataatIndex (LocalVariables|GetLocalIndex)))))
    (Utilities|IsValid _returnvalue
      (:Is%20Valid
        (Default|UseItem _returnvalue))
      (:Is%20Not%20Valid
        (bind _returnvalue_2 (Game|SpawnActorfromClass (.Item (CallFunction|GetItemDataatIndex (LocalVariables|GetLocalIndex))) (Math|Transform|MakeTransform "0, 0, 0" "0, 0, 0" "1.000000,1.000000,1.000000") "Undefined" 0 0))
        (Default|UseItem _returnvalue_2)))
    (bind _asrpg_main_character (Utilities|Casting|CastToRPG_MainCharacter (Game|GetPlayerCharacter 0)))
    (switch Utilities|FlowControl|Switch|SwitchonCharacterStats (Variables|/Game/_Game/Characters/Player/RPG_MainCharacter.RPG_MainCharacter_C|GetCharacterStats _asrpg_main_character)
      (:NewEnumerator0
        (CallFunction|RemoveItem (LocalVariables|GetLocalIndex) :!label _label))
      (:NewEnumerator1
        (if (< (Variables|/Game/_Game/Characters/Player/RPG_MainCharacter.RPG_MainCharacter_C|GetCurrentHealth (Variables|Default|GetPlayerRef)) 1e+02)
          (CallFunction|RemoveItem (LocalVariables|GetLocalIndex))))
      (:NewEnumerator2
        (goto _label)))))

(fn RemoveItem
  (params (Index :type Integer))
  (bind _output_get (LocalVariables|SetLocalIndex Index))
  (if (> (.Amount (CallFunction|GetItemDataatIndex _output_get)) 1)
    (Utilities|Array|SetArrayElem (Variables|Default|GetInventorySlots) (LocalVariables|GetLocalIndex) (Utilities|Struct|MakeSInventoryItems (.Item (CallFunction|GetItemDataatIndex _output_get)) (- (.Amount (CallFunction|GetItemDataatIndex _output_get)) 1)))
    (else
      (Utilities|Array|SetArrayElem (Variables|Default|GetInventorySlots) (LocalVariables|GetLocalIndex) (Utilities|Struct|MakeSInventoryItems 0 0))))
  (CallFunction|UpdateInventorySlot (LocalVariables|GetLocalIndex))
  (Default|CloseDropDownMenu (Variables|/Game/_Game/UI/Menu/W_SelectionMenu.W_SelectionMenu_C|GetW_Inventory (Variables|Default|GetSelectionMenuRef))))

(fn DropOneItem
  (params (Index :type Integer))
  (bind _playerref (Variables|Default|GetPlayerRef))
  (bind _sprite (Variables|/Script/Paper2D.PaperCharacter|GetSprite _playerref))
  (bind _returnvalue (Transformation|GetWorldLocation _sprite))
  (bind _output_get (LocalVariables|SetLocalIndex Index))
  (LocalVariables|SetLocalItem (.Item (CallFunction|GetItemDataatIndex _output_get)))
  (LocalVariables|SetLocalAmount (.Amount (CallFunction|GetItemDataatIndex _output_get)))
  (if (> (LocalVariables|GetLocalAmount) 0)
    (if (not (.KeyItem (Utilities|Struct|BreakSItemData (.ItemData (Utilities|GetClassDefaults (LocalVariables|GetLocalItem))))))
      (CallFunction|RemoveItem (LocalVariables|GetLocalIndex))
      (bind _output_get_2 (LocalVariables|SetLocalAmount (- (LocalVariables|GetLocalAmount) (LocalVariables|GetLocalAmount))))
      (Math|Integer|IncrementInt _output_get_2
        (:%20%20
          (Default|CloseDropDownMenu (Variables|/Game/_Game/UI/Menu/W_SelectionMenu.W_SelectionMenu_C|GetW_Inventory (Variables|Default|GetSelectionMenuRef)))
          (bind (_outhit _returnvalue_2) (Collision|LineTraceByChannel _returnvalue (+ _returnvalue (* (Math|Vector|GetForwardVector _sprite) 25.0)) "TraceTypeQuery1" false 0 "None"))
          (bind _returnvalue_3 (Actor|GetActorOfClass (.PickupActor (Utilities|Struct|BreakSItemData (.ItemData (Utilities|GetClassDefaults (LocalVariables|GetLocalItem)))))))
          (Utilities|IsValid _returnvalue_3
            (:Is%20Valid
              (Variables|/Game/_Game/Blueprints/Inventory/InventoryItems/PickupActors/BP_PickupActorMaster.BP_PickupActorMaster_C|SetAmount _returnvalue_3 (+ (LocalVariables|GetLocalAmount) (Variables|/Game/_Game/Blueprints/Inventory/InventoryItems/PickupActors/BP_PickupActorMaster.BP_PickupActorMaster_C|GetAmount _returnvalue_3))))
            (:Is%20Not%20Valid
              (bind _returnvalue_4 (Game|SpawnActorfromClass (.pickupactor (.ItemData (Utilities|GetClassDefaults (LocalVariables|GetLocalItem)))) (Math|Transform|MakeTransform (select _returnvalue_2 (.Location (Collision|BreakHitResult _outhit)) (.TraceEnd (Collision|BreakHitResult _outhit))) "0, 0, 0" "1.000000,1.000000,1.000000") "Undefined" 0 0 "ItemMaster" 0))
              (bind _asrpg_game_instance (Utilities|Casting|CastToRPG_GameInstance (Game|GetGameInstance)))
              (Variables|/Game/_Game/Config/GameInstance/RPG_GameInstance.RPG_GameInstance_C|SetCanBeDestroyed _asrpg_game_instance false)
              (Variables|/Game/_Game/Blueprints/Inventory/InventoryItems/PickupActors/BP_PickupActorMaster.BP_PickupActorMaster_C|SetAmount _returnvalue_4 (LocalVariables|GetLocalAmount))
              (Physics|SetSimulatePhysics (Variables|/Game/_Game/Blueprints/Inventory/InventoryItems/PickupActors/BP_PickupActorMaster.BP_PickupActorMaster_C|GetPaperSprite _returnvalue_4) true)
              (Collision|SetCollisionEnabled (Variables|/Game/_Game/Blueprints/Inventory/InventoryItems/PickupActors/BP_PickupActorMaster.BP_PickupActorMaster_C|GetPaperSprite _returnvalue_4) "QueryAndPhysics")
              (Collision|SetCollisionResponsetoChannel (Variables|/Game/_Game/Blueprints/Inventory/InventoryItems/PickupActors/BP_PickupActorMaster.BP_PickupActorMaster_C|GetPaperSprite _returnvalue_4) "ECC_Pawn" "ECR_Ignore")
              (CallFunction|UpdateInventorySlot (LocalVariables|GetLocalIndex)))))))))

(fn DropAll
  (params (Index :type Integer))
  (bind _playerref (Variables|Default|GetPlayerRef))
  (bind _sprite (Variables|/Script/Paper2D.PaperCharacter|GetSprite _playerref))
  (bind _returnvalue (Transformation|GetWorldLocation _sprite))
  (bind _output_get (LocalVariables|SetLocalIndex Index))
  (LocalVariables|SetLocalItem (.Item (CallFunction|GetItemDataatIndex _output_get)))
  (LocalVariables|SetLocalAmount (.Amount (CallFunction|GetItemDataatIndex _output_get)))
  (if (> (LocalVariables|GetLocalAmount) 0)
    (CallFunction|RemoveItem (LocalVariables|GetLocalIndex))
    (for _index (range 0 (- (LocalVariables|GetLocalAmount) 1))
      (CallFunction|RemoveItem (LocalVariables|GetLocalIndex)))
    (Default|CloseDropDownMenu (Variables|/Game/_Game/UI/Menu/W_SelectionMenu.W_SelectionMenu_C|GetW_Inventory (Variables|Default|GetSelectionMenuRef)))
    (bind (_outhit _returnvalue_2) (Collision|LineTraceByChannel _returnvalue (+ _returnvalue (* (Math|Vector|GetForwardVector _sprite) 25.0)) "TraceTypeQuery1" false 0 "None"))
    (bind _returnvalue_3 (Actor|GetActorOfClass (.PickupActor (Utilities|Struct|BreakSItemData (.ItemData (Utilities|GetClassDefaults (LocalVariables|GetLocalItem)))))))
    (Utilities|IsValid _returnvalue_3
      (:Is%20Valid
        (Variables|/Game/_Game/Blueprints/Inventory/InventoryItems/PickupActors/BP_PickupActorMaster.BP_PickupActorMaster_C|SetAmount _returnvalue_3 (+ (LocalVariables|GetLocalAmount) (Variables|/Game/_Game/Blueprints/Inventory/InventoryItems/PickupActors/BP_PickupActorMaster.BP_PickupActorMaster_C|GetAmount _returnvalue_3))))
      (:Is%20Not%20Valid
        (bind _returnvalue_4 (Game|SpawnActorfromClass (.pickupactor (.ItemData (Utilities|GetClassDefaults (LocalVariables|GetLocalItem)))) (Math|Transform|MakeTransform (select _returnvalue_2 (.Location (Collision|BreakHitResult _outhit)) (.TraceEnd (Collision|BreakHitResult _outhit))) "0, 0, 0" "1.000000,1.000000,1.000000") "Undefined" 0 0 "ItemMaster" 0))
        (Variables|/Game/_Game/Blueprints/Inventory/InventoryItems/PickupActors/BP_PickupActorMaster.BP_PickupActorMaster_C|SetAmount _returnvalue_4 (LocalVariables|GetLocalAmount))
        (Physics|SetSimulatePhysics (Variables|/Game/_Game/Blueprints/Inventory/InventoryItems/PickupActors/BP_PickupActorMaster.BP_PickupActorMaster_C|GetPaperSprite _returnvalue_4) true)
        (Collision|SetCollisionEnabled (Variables|/Game/_Game/Blueprints/Inventory/InventoryItems/PickupActors/BP_PickupActorMaster.BP_PickupActorMaster_C|GetPaperSprite _returnvalue_4) "QueryAndPhysics")
        (Collision|SetCollisionResponsetoChannel (Variables|/Game/_Game/Blueprints/Inventory/InventoryItems/PickupActors/BP_PickupActorMaster.BP_PickupActorMaster_C|GetPaperSprite _returnvalue_4) "ECC_Pawn" "ECR_Ignore")))))

(fn AddIteminEquipSlot
  (params (Item :type BP%20Inventory%20Item%20Master%20Class%20Reference) (Amount :type Integer))
  (bind (_success _index) (CallFunction|CheckforEmptyEquipSlot))
  (LocalVariables|SetLocalItem Item)
  (LocalVariables|SetLocalAmount Amount)
  (LocalVariables|SetLocalMaxStackAmount (.MaxStackAmount (Utilities|Struct|BreakSItemData (.ItemData (Utilities|GetClassDefaults (LocalVariables|GetLocalItem))))))
  (if _success
    (LocalVariables|SetLocalIndex _index)
    (Utilities|Array|SetArrayElem (Variables|Default|GetEquipSlots) (LocalVariables|GetLocalIndex) (Utilities|Struct|MakeSInventoryItems (LocalVariables|GetLocalItem) (LocalVariables|GetLocalAmount)))
    (CallFunction|UpdateEquipSlot (LocalVariables|GetLocalIndex))
    (return true)
    (else
      (Development|PrintText "No free slots!")
      (return false))))

(fn CheckforEmptyEquipSlot
  (bind (_array_element _array_index) (Utilities|Array|ForEachLoopwithBreak (Variables|Default|GetEquipSlots) :!label _label)
    (:LoopBody
      (if (Utilities|IsValidClass (.Item (Utilities|Struct|BreakSInventoryItems _array_element)))
        (LocalVariables|SetLocalSuccess false)
        (else
          (LocalVariables|SetLocalSuccess true)
          (LocalVariables|SetLocalIndex _array_index)
          (goto _label Break))))
    (:Completed
      (return (LocalVariables|GetLocalSuccess) (LocalVariables|GetLocalIndex)))))

(fn GetEquiItemDataatIndex
  (params (Index :type Integer))
  (bind _equipslots (Variables|Default|GetEquipSlots))
  (bind _output (Utilities|Array|Get(acopy) _equipslots Index))
  (bind (_item _amount) (Utilities|Struct|BreakSInventoryItems _output))
  (return _item _amount))

(fn UpdateEquipSlot
  (params (Index :type Integer))
  (Default|UpdateSlot (Utilities|Array|Get(acopy) (Variables|/Game/_Game/UI/Inventory/W_EquipSlotGrid.W_EquipSlotGrid_C|GetEquipSlotsArray (Variables|/Game/_Game/UI/Inventory/W_Inventory.W_Inventory_C|GetW_EquipSlotGrid (Variables|/Game/_Game/UI/Menu/W_SelectionMenu.W_SelectionMenu_C|GetW_Inventory (Variables|/Game/_Game/Config/PlayerController/RPGController.RPGController_C|GetSelectionMenuRef (.AsRPGController (Utilities|Casting|CastToRPGController (Game|GetPlayerController 0))))))) Index)))

(fn EquipItem
  (params (ItemToEquip :type BP%20Inventory%20Item%20Master%20Class%20Reference) (SwitchToItem :type BP%20Inventory%20Item%20Master%20Class%20Reference) (Slot%20Index :type Integer) (Equip%20Slot%20Index :type Integer))
  (bind (_success _index) (CallFunction|CheckforEmptyEquipSlot))
  (bind _playerref (Variables|Default|GetPlayerRef))
  (LocalVariables|SetLocalItemToEquip ItemToEquip)
  (LocalVariables|SetLocalEquippedItem SwitchToItem)
  (LocalVariables|SetLocalIndex Slot%20Index)
  (if _success
    (LocalVariables|SetLocalEquipIndex _index)
    (CallFunction|RemoveItem (LocalVariables|GetLocalIndex))
    (CallFunction|AddIteminEquipSlot (LocalVariables|GetLocalItemToEquip) 1)
    (CallFunction|UpdateEquipSlot (LocalVariables|GetLocalEquipIndex))
    (CallFunction|UpdateInventorySlot (LocalVariables|GetLocalIndex))
    (Default|GetDamagetoAdd _playerref (LocalVariables|GetLocalEquipIndex))
    (Default|GetShieldtoAdd _playerref (LocalVariables|GetLocalEquipIndex))
    (else
      (Development|PrintText "Already in Use!"))))

(fn SwitchItem
  (params (ItemToSwitch :type BP%20Inventory%20Item%20Master%20Class%20Reference) (SwitchToItem :type BP%20Inventory%20Item%20Master%20Class%20Reference))
  (bind _output_get (LocalVariables|SetLocalPreviousItem ItemToSwitch))
  (return _output_get SwitchToItem))

(fn RemoveItemEquipped
  (params (Index :type Integer))
  (LocalVariables|SetLocalIndex Index)
  (Utilities|Array|SetArrayElem (Variables|Default|GetEquipSlots) (LocalVariables|GetLocalIndex) (Utilities|Struct|MakeSInventoryItems 0 0))
  (CallFunction|UpdateInventorySlot (LocalVariables|GetLocalIndex))
  (Default|CloseDropDownMenu (Variables|/Game/_Game/UI/Menu/W_SelectionMenu.W_SelectionMenu_C|GetW_Inventory (Variables|Default|GetSelectionMenuRef))))

(fn UnEquipItem
  (params (ItemToEquip :type BP%20Inventory%20Item%20Master%20Class%20Reference) (SwitchToItem :type BP%20Inventory%20Item%20Master%20Class%20Reference) (Slot%20Index :type Integer) (Equip%20Slot%20Index :type Integer))
  (bind _playerref (Variables|Default|GetPlayerRef))
  (LocalVariables|SetLocalItemToEquip ItemToEquip)
  (LocalVariables|SetLocalEquippedItem SwitchToItem)
  (LocalVariables|SetLocalIndex Slot%20Index)
  (LocalVariables|SetLocalEquipIndex Equip%20Slot%20Index)
  (bind (_previousitem _nextitem) (CallFunction|SwitchItem (LocalVariables|GetLocalItemToEquip) (LocalVariables|GetLocalEquippedItem)))
  (LocalVariables|SetLocalPreviousItem _previousitem)
  (LocalVariables|SetLocalNextItem _nextitem)
  (CallFunction|UpdateInventorySlot (LocalVariables|GetLocalIndex))
  (Default|GetDamagetoRemove _playerref (LocalVariables|GetLocalEquipIndex))
  (Default|GetShieldtoRemove _playerref (LocalVariables|GetLocalEquipIndex))
  (CallFunction|AddItem (LocalVariables|GetLocalNextItem) 1)
  (CallFunction|RemoveItemEquipped (LocalVariables|GetLocalEquipIndex))
  (CallFunction|UpdateEquipSlot (LocalVariables|GetLocalEquipIndex))
  (CallFunction|UpdateInventorySlot (LocalVariables|GetLocalIndex))
  (LocalVariables|SetLocalNextItem (LocalVariables|GetLocalItemToEquip)))

(fn SellItem
  (params (Index :type Integer))
  (LocalVariables|SetLocalIndex Index)
  (Utilities|Array|SetArrayElem (Variables|Default|GetInventorySlots) (LocalVariables|GetLocalIndex) (Utilities|Struct|MakeSInventoryItems 0 0))
  (CallFunction|UpdateInventorySlot (LocalVariables|GetLocalIndex))
  (Default|CloseDropDownMenu (Variables|/Game/_Game/UI/Menu/W_SelectionMenu.W_SelectionMenu_C|GetW_Inventory (Variables|Default|GetSelectionMenuRef))))